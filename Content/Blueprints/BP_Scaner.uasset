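; BP_Scaner is a scanner actor that shows whether a BP_GoodMoney object placed in it is good or bad.
; A Box overlap casts the entering actor to BP_GoodMoney, reads its Good flag and, after a short delay, turns the PointLight green or red.
; Any actor leaving the box resets the light to near white, without cancelling a pending color change.
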(event `self.Box.OnComponentBeginOverlap`
  (params (OverlappedComponent :type "PrimitiveComponent Object Reference") (OtherActor :type "Actor Object Reference") (OtherComp :type "PrimitiveComponent Object Reference") (OtherBodyIndex :type Integer) (bFromSweep :type Boolean) (SweepResult :type "HitResult Structure (by ref)"))
  (bind _asbp_good_money (cast `/Game/Blueprints/BP_GoodMoney` OtherActor))
  (if (`/Game/Blueprints/BP_GoodMoney.Good?` _asbp_good_money)
    (`KismetSystemLibrary.Delay` 0.5)
    (`LightComponent.SetLightColor` (`self.PointLight`) (struct :`R` 0.121442 :`G` 0.666667 :`B` 0.131792 :`A` 1.0) true)
    (else
      (`KismetSystemLibrary.Delay` 0.5)
      (`LightComponent.SetLightColor` (`self.PointLight`) (struct :`R` 0.908333 :`G` 0.093974 :`B` 0.05782 :`A` 1.0) true))))

(event `self.Box.OnComponentEndOverlap`
  (params (OverlappedComponent :type "PrimitiveComponent Object Reference") (OtherActor :type "Actor Object Reference") (OtherComp :type "PrimitiveComponent Object Reference") (OtherBodyIndex :type Integer))
  (`LightComponent.SetLightColor` (`self.PointLight`) (struct :`R` 1.0 :`G` 0.987676 :`B` 0.979482 :`A` 1.0) true))

(fn `UserConstructionScript`)