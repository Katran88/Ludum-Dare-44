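; An ATM actor with a swinging door that takes in money actors and displays a running balance.
; The outer collision shows an open-door widget and permits opening, then removes it on exit and calls OpenDoor after a short delay to close.
; OpenDoor plays or reverses a timeline that rotates the cylinder.
; The inner collision casts entering actors to BP_GoodMoney after a delay, adding or subtracting their value by the Good flag.
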(event `self.Collision_Out.OnComponentBeginOverlap`
  (params (OverlappedComponent :type "PrimitiveComponent Object Reference") (OtherActor :type "Actor Object Reference") (OtherComp :type "PrimitiveComponent Object Reference") (OtherBodyIndex :type Integer) (bFromSweep :type Boolean) (SweepResult :type "HitResult Structure (by ref)"))
  ;[1 1 1] Add/remove Widget
  (bind _returnvalue (`|CreateWidget` "/Game/Widgets/W_OpenDoor.W_OpenDoor_C" (`GameplayStatics.GetPlayerController` 0)))
  (bind _output_get (set `self.W_open` _returnvalue))
  (`UserWidget.AddToViewport` _output_get 0)
  (set `self.CanOpen` true))

(event `self.Collision_Out.OnComponentEndOverlap`
  (params (OverlappedComponent :type "PrimitiveComponent Object Reference") (OtherActor :type "Actor Object Reference") (OtherComp :type "PrimitiveComponent Object Reference") (OtherBodyIndex :type Integer))
  (bind _w_open (`self.W_open`))
  ;[1 1 1] Add/remove Widget
  (`/Engine/EditorBlueprintResources/StandardMacros.IsValid` _w_open
    (:`Is Valid`
      (`Widget.RemoveFromParent` _w_open))
    (:`Is Not Valid`
      _))
  (set `self.CanOpen` false)
  (`KismetSystemLibrary.Delay` 0.5)
  (`self.OpenDoor`))

(event `OpenDoor`
  ;[1 1 1] OpenDoor
  (if (`self.CanOpen`)
    (bind (_direction _value) (`Timeline|Time` :!label _label)
      (:`Update`
        (`SceneComponent.K2_SetWorldRotation` (`self.Cylinder`) (`KismetMathLibrary.RLerp` (struct :`Roll` 90.0) (struct :`Pitch` 35.0 :`Roll` 90.0) _value) false false)))
    (else
      (goto _label :!via `Reverse`))))

(event `self.Collision_inside.OnComponentBeginOverlap`
  (params (OverlappedComponent :type "PrimitiveComponent Object Reference") (OtherActor :type "Actor Object Reference") (OtherComp :type "PrimitiveComponent Object Reference") (OtherBodyIndex :type Integer) (bFromSweep :type Boolean) (SweepResult :type "HitResult Structure (by ref)"))
  ;[1 1 1] Balance
  (`KismetSystemLibrary.Delay` 1.0)
  (set `self.Money` (cast `/Game/Blueprints/BP_GoodMoney` OtherActor :!pure true))
  (if (`/Game/Blueprints/BP_GoodMoney.Good?` (`self.Money`))
    (bind _output_get (set `self.Balance` (+ (`/Game/Blueprints/BP_GoodMoney.Value` (`self.Money`)) (`self.Balance`))))
    (`TextRenderComponent.K2_SetText` (`self.Balance_value`) (`KismetTextLibrary.Conv_IntToText` _output_get))
    (else
      (bind _output_get_2 (set `self.Balance` (- (`self.Balance`) (`/Game/Blueprints/BP_GoodMoney.Value` (`self.Money`)))))
      (`TextRenderComponent.K2_SetText` (`self.Balance_value`) (`KismetTextLibrary.Conv_IntToText` _output_get_2)))))

(fn `UserConstructionScript`)